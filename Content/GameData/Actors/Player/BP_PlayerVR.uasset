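; VR player Blueprint that lets the user pick up and drop one physics object at a time with the left motion controller.
; BeginPlay sets the tracking origin to Eye when an HMD is enabled, although the graph's comment says floor level.
; GrabLeft line-traces forward from the controller, disables physics on the hit component and snaps its actor to HeldObjectPos.
; Release detaches the actor and restores physics.
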(event `self.ReceiveBeginPlay`
  ;[1 1 1] Set Cam tracking origin to floor level ( Allows for Variable User Height)
  (if (`HeadMountedDisplayFunctionLibrary.IsHeadMountedDisplayEnabled`)
    (`HeadMountedDisplayFunctionLibrary.SetTrackingOrigin` "Eye")))

(event `InputAction|GrabLeft`
  (params (Key :type "Key Structure"))
  ;[1 1 1] Motion Controller Input (Grip and Drop Left Hand) Taken from: https://docs.unrealengine.com/5.0/en-US/using-motion-controllers-in-unreal-engine/ . Ideally will be in c++ but VS is causing issues with motion controllers so BP only player for now
  ;;[1 1 1] Allow the Player to only pick up one object
  (:`Pressed`
    (if (not (`self.bIsHoldingObject`))
      (`self.PickUp`)))
  (:`Released`
    (`self.Drop`)))

(event `PickUp`
  (bind _hit_component (`self.Hit Component`))
  (bind _mcleft (`self.MCLeft`))
  (bind _returnvalue (`SceneComponent.K2_GetComponentLocation` _mcleft))
  ;[1 1 1] Motion Controller Input (Grip and Drop Left Hand) Taken from: https://docs.unrealengine.com/5.0/en-US/using-motion-controllers-in-unreal-engine/ . Ideally will be in c++ but VS is causing issues with motion controllers so BP only player for now
  ;;[1 1 1] Pick Up event
  (bind (_outhit _returnvalue_2) (`KismetSystemLibrary.LineTraceSingleForObjects` _returnvalue (+ _returnvalue (* (`SceneComponent.GetForwardVector` _mcleft) 1000.0)) (`|MakeArray` "ObjectTypeQuery4" :!type "EObjectTypeQuery Enum")))
  (if _returnvalue_2
    (bind (_bblockinghit _binitialoverlap _time _distance _location _impactpoint _normal _impactnormal _physmat _hitactor _hitcomponent) (`GameplayStatics.BreakHitResult` _outhit))
    ;;[1 1 1] If targeted component simulates physics (can be picked up) = true
    (set `self.Hit Component` _hitcomponent)
    (if (`SceneComponent.IsAnySimulatingPhysics` _hit_component)
      ;;[1 1 1] Attach to hand
      (bind _output_get (set `self.PickedUpObject` _hitactor))
      (`PrimitiveComponent.SetSimulatePhysics` _hit_component false)
      (`self.K2_AttachToComponent` _output_get (`self.HeldObjectPos`) "None" "SnapToTarget" "SnapToTarget" "KeepWorld" true)
      (set `self.bIsHoldingObject` true))))

(event `Drop`
  (bind _pickedupobject (`self.PickedUpObject`))
  (bind _hit_component (`self.Hit Component`))
  ;[1 1 1] Motion Controller Input (Grip and Drop Left Hand) Taken from: https://docs.unrealengine.com/5.0/en-US/using-motion-controllers-in-unreal-engine/ . Ideally will be in c++ but VS is causing issues with motion controllers so BP only player for now
  (`/Engine/EditorBlueprintResources/StandardMacros.IsValid` _pickedupobject
    (:`Is Valid`
      (`self.K2_DetachFromActor` _pickedupobject "KeepWorld" "KeepWorld" "KeepWorld")
      (`/Engine/EditorBlueprintResources/StandardMacros.IsValid` _hit_component
        (:`Is Valid`
          (`PrimitiveComponent.SetSimulatePhysics` _hit_component true)
          (set `self.bIsHoldingObject` false)
          (set `self.Hit Component` null)
          (set `self.PickedUpObject` null))))))

(fn `UserConstructionScript`)